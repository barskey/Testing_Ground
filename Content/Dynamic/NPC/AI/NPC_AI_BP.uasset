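; AI controller for patrolling guard NPCs, running the guard behavior tree on the patrol blackboard at BeginPlay.
; AI perception writes any sensed actor not tagged "Enemy" to the blackboard's enemy key and clears that key when sensing is lost.
; Every tick it sets the controlled PatrollingGuard2's Aiming flag according to whether the controller has a valid focus actor.
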(event OnTargetPerceptionUpdated(AIPerception)
  (params (Actor :type Actor%20Object%20Reference) (Stimulus :type AI%20Stimulus%20Structure))
  (bind _enemykey (Variables|Default|GetEnemyKey))
  (if (not (Actor|ActorHasTag Actor "Enemy"))
    (if (.bSuccessfullySensed (Utilities|Struct|BreakAIStimulus Stimulus))
      (AI|Components|Blackboard|SetValueasObject (stale EventBeginPlay _blackboardcomponent) _enemykey Actor)
      (else
        (AI|Components|Blackboard|ClearValue (stale EventBeginPlay _blackboardcomponent) _enemykey)))))

(event EventBeginPlay
  (bind _blackboardcomponent (Class|AIController|UseBlackboard "/Game/Dynamic/NPC/AI/PatrolData.PatrolData"))
  (AI|RunBehaviorTree "/Game/Dynamic/NPC/AI/GuardBehavior.GuardBehavior"))

(event EventTick
  (params (DeltaSeconds :type Float%20%28single-precision%29))
  (bind _aspatrolling_guard_2 (Utilities|Casting|CastToPatrollingGuard2 (Pawn|GetControlledPawn)))
  (Variables|/Game/Dynamic/NPC/Behavior/PatrollingGuard2.PatrollingGuard2_C|SetAiming _aspatrolling_guard_2 (Utilities|IsValid (Class|AIController|GetFocusActor))))

(fn ConstructionScript)